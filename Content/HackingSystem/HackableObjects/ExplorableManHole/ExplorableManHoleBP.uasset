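; Hackable manhole actor that explodes when the player successfully hacks it.
; Targeting shows a widget and a beam from the manhole to the player's pawn, with hack progress driving the widget's progress-bar material.
; Success removes the targeting components, plays explosion effects, disables manhole physics simulation, then applies a random, mostly upward impulse.
; A looping timer adds random spin until the manhole registers a hit.
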(event `self.ReceiveBeginPlay`
  (`ParticleSystemComponent.SetBeamSourcePoint` (`self.TargettedParrticules`) 0 (`SceneComponent.K2_GetComponentLocation` (`self.ManHole`)) 0))

(event `/Game/HackingSystem/HackableObjects/HackableEventsBPI.OnObjectTargetted`
  (`SceneComponent.SetVisibility` (`self.TargetWidget`) true false)
  (`ParticleSystemComponent.SetBeamEndPoint` (`self.TargettedParrticules`) 0 (`self.K2_GetActorLocation` (`Controller.K2_GetPawn` (`GameplayStatics.GetPlayerController` 0))))
  (`SceneComponent.SetVisibility` (`self.TargettedParrticules`) true false))

(event `/Game/HackingSystem/HackableObjects/HackableEventsBPI.OnObjectUnTargetted`
  (`SceneComponent.SetVisibility` (`self.TargettedParrticules`) false false)
  (`SceneComponent.SetVisibility` (`self.TargetWidget`) false false))

(event `/Game/HackingSystem/HackableObjects/HackableEventsBPI.UpdateObjectHackingProgress`
  (params (`Progress Value` :type "Float (double-precision)"))
  (bind _asfocus_object (cast `/Game/HackingSystem/Visual/FocusObject` (`WidgetComponent.GetUserWidgetObject` (`self.TargetWidget`))))
  (bind _progressbar (`/Game/HackingSystem/Visual/FocusObject.ProgressBar` _asfocus_object))
  (bind _returnvalue (`Image.GetDynamicMaterial` _progressbar))
  (`Image.SetBrushFromMaterial` _progressbar _returnvalue)
  (`MaterialInstanceDynamic.SetScalarParameterValue` _returnvalue "Progress" `Progress Value`))

(event `/Game/HackingSystem/HackableObjects/HackableEventsBPI.OnSuccessFullHack`
  (bind _returnvalue (`self.K2_GetActorLocation`))
  (bind _returnvalue_2 (`KismetMathLibrary.RandomFloatInRange` 50.0 150.0))
  (bind _manhole (`self.ManHole`))
  (`PrimitiveComponent.SetCollisionResponseToChannel` (`self.Sphere`) "ECC_Visibility" "ECR_Ignore")
  (`ActorComponent.K2_DestroyComponent` (`self.TargetWidget`))
  (`ActorComponent.K2_DestroyComponent` (`self.TargettedParrticules`))
  (`KismetSystemLibrary.PrintString` "gg" true true (struct :`R` 1.0 :`B` 0.152706 :`A` 1.0))
  (`GameplayStatics.SpawnEmitterAtLocation` "/Game/StarterContent/Particles/P_Explosion.P_Explosion" _returnvalue (struct) (4.0 4.0 4.0))
  (`GameplayStatics.PlaySoundAtLocation` "/Game/StarterContent/Audio/Explosion01.Explosion01" _returnvalue (struct) 1.0 1.0 0.0 null null null null)
  (`PrimitiveComponent.SetSimulatePhysics` _manhole false)
  (`PrimitiveComponent.AddImpulse` _manhole (`KismetMathLibrary.MakeVector` _returnvalue_2 _returnvalue_2 (`KismetMathLibrary.RandomFloatInRange` 750.0 950.0)) "None" true)
  (bind _returnvalue_3 (`KismetSystemLibrary.K2_SetTimerDelegate` (delegate `Rotate ManHole`) 0.01 true))
  (`KismetSystemLibrary.K2_ClearAndInvalidateTimerHandle` _returnvalue_3 :!label _label))

(event `Rotate ManHole`
  (bind _returnvalue (`KismetMathLibrary.RandomFloatInRange` 0.0 5.0))
  (`SceneComponent.K2_AddLocalRotation` (`self.ManHole`) (`KismetMathLibrary.MakeRotator` _returnvalue _returnvalue _returnvalue) false false))

(event `self.ManHole.OnComponentHit`
  (params (HitComponent :type "PrimitiveComponent Object Reference") (OtherActor :type "Actor Object Reference") (OtherComp :type "PrimitiveComponent Object Reference") (NormalImpulse :type "Vector Structure") (Hit :type "HitResult Structure (by ref)"))
  (goto _label))

(fn `UserConstructionScript`)